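; Player Blueprint for a Crossy Road-style chicken that hops in fixed grid steps and tracks distance and coins.
; Move inputs call CheckValidity to gate on death, blocking and jumping and set facing, then jump, offset the capsule with sweep and reset the idle timer.
; Tick creeps the camera forward, offsets it when the player gets ahead, and flags DeathByEagle after 600 idle ticks.
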(event `self.ReceiveTick`
  (params (DeltaSeconds :type "Float (single-precision)"))
  ;[1 1 1] Trigger Idle Death
  (`|ExecutionSequence`
    (:`then_0`
      (bind _result (`/Engine/EditorBlueprintResources/StandardMacros.IncrementInt` (`self.Timer`))
        (:`  `
          (if (== _result 600)
            (set `self.DeathByEagle` true)))))
    (:`then_1`
      (`self.CheckCamera`)
      ;[1 1 1] Slow Camera Panning
      (`SceneComponent.K2_AddWorldOffset` (`self.Camera`) (0.3 0.0 0.0) false false))))

(event `InputAction|Move Forward`
  (params (Key :type "Key Structure"))
  ;[1 1 1] Character Movement
  (:`Pressed`
    (bind _valid (`self.CheckValidity` (`self.R_Forward`)))
    (if _valid
      (set `self.IsJumping` true)
      (`self.Jump`)
      (`SceneComponent.K2_AddWorldOffset` (`self.CapsuleComponent`) (110.0 0.0 0.0) true false)
      (`self.CheckLocationHigh`))
    (`KismetSystemLibrary.Delay` 0.1)
    (`self.UpdateAfterJump`)))

(event `InputAction|Move Left`
  (params (Key :type "Key Structure"))
  ;[1 1 1] Character Movement
  (:`Pressed`
    (bind _valid (`self.CheckValidity` (`self.R_Left`)))
    (if _valid
      (set `self.IsJumping` true)
      (`self.Jump`)
      (`SceneComponent.K2_AddWorldOffset` (`self.CapsuleComponent`) (0.0 -110.0 0.0) true false))
    (`KismetSystemLibrary.Delay` 0.1)
    (`self.UpdateAfterJump`)))

(event `InputAction|Move Backward`
  (params (Key :type "Key Structure"))
  ;[1 1 1] Character Movement
  (:`Pressed`
    (bind _valid (`self.CheckValidity` (`self.R_Backward`)))
    (if _valid
      (set `self.IsJumping` true)
      (`self.Jump`)
      (`SceneComponent.K2_AddWorldOffset` (`self.CapsuleComponent`) (-110.0 0.0 0.0) true false))
    (`KismetSystemLibrary.Delay` 0.1)
    (`self.UpdateAfterJump`)))

(event `InputAction|Move Right`
  (params (Key :type "Key Structure"))
  ;[1 1 1] Character Movement
  (:`Pressed`
    (bind _valid (`self.CheckValidity` (`self.R_Right`)))
    (if _valid
      (set `self.IsJumping` true)
      (`self.Jump`)
      (`SceneComponent.K2_AddWorldOffset` (`self.CapsuleComponent`) (0.0 110.0 0.0) true false))
    (`KismetSystemLibrary.Delay` 0.1)
    (`self.UpdateAfterJump`)))

(event `self.ReceiveBeginPlay`
  ;[1 1 1] Camera Initialization
  (set `self.R_Forward` (`SceneComponent.K2_GetComponentRotation` (`self.StaticMesh`)))
  (`SceneComponent.SetAbsolute` (`self.Camera`) false false false))

(event `self.ReceiveHit`
  (params (MyComp :type "PrimitiveComponent Object Reference") (Other :type "Actor Object Reference") (OtherComp :type "PrimitiveComponent Object Reference") (bSelfMoved :type Boolean) (HitLocation :type "Vector Structure") (HitNormal :type "Vector Structure") (NormalImpulse :type "Vector Structure") (Hit :type "HitResult Structure (by ref)"))
  ;[1 1 1] Collision Handling
  (switch `int` (`self.SwitchForDeath`)))

(fn `CheckCamera`
  (bind _returnvalue_x (`KismetMathLibrary.BreakVector` (`SceneComponent.K2_GetComponentLocation` (`self.StaticMesh`))))
  (bind _returnvalue_x_2 (`KismetMathLibrary.BreakVector` (`SceneComponent.K2_GetComponentLocation` (`self.Camera`))))
  (if (> _returnvalue_x _returnvalue_x_2)
    (`SceneComponent.K2_AddWorldOffset` (`self.Camera`) (`SceneComponent.K2_GetComponentLocation` (`self.StaticMesh`)) false false)))

(fn `CheckLocationHigh`
  (bind _furthestlocation_x (`KismetMathLibrary.BreakVector` (`self.FurthestLocation`)))
  (bind _returnvalue_x (`KismetMathLibrary.BreakVector` (`SceneComponent.K2_GetComponentLocation` (`self.StaticMesh`))))
  (if (> _returnvalue_x _furthestlocation_x)
    (`self.IncrementDistance`)))

(fn `CheckValidity`
  (params (`Chicken Orientation` :type "Rotator Structure"))
  (returns (Valid :type Boolean) (Invalid :type Boolean))
  (bind _staticmesh (`self.StaticMesh`))
  (if (`self.IsDead`)
    (return false true)
    (elif (`self.IsBlockedLeft`)
      (return false true)
      (elif (`self.IsBlockedRight`)
        (return false true)
        (elif (`self.IsJumping`)
          (return false true)
          (elif (not (== (`SceneComponent.K2_GetComponentRotation` _staticmesh) `Chicken Orientation`))
            (`SceneComponent.K2_SetWorldRotation` _staticmesh `Chicken Orientation` false false)
            (set `self.PreviousLocation` (`SceneComponent.K2_GetComponentLocation` (`self.CapsuleComponent`)))
            (return true false)))))))

(fn `IncrementCoin`
  (`/Engine/EditorBlueprintResources/StandardMacros.IncrementInt` (`self.Coins`)))

(fn `IncrementDistance`
  (if (not (`self.IsDead`))
    (`/Engine/EditorBlueprintResources/StandardMacros.IncrementInt` (`self.Distance`))))

(fn `UpdateAfterJump`
  (set `self.IsJumping` false)
  (set `self.Timer` 0))

(fn `UserConstructionScript`)