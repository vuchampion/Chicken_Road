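; Terrain generator actor that builds a continuous run of Terrain lanes, starting at an offset from the player pawn.
; On BeginPlay it lays a starting strip of type 0, chaining each lane to the previous one's SpawnPoint, then adds random chunks until LaneMax.
; Each chunk repeats one random terrain type for a short random run.
; RemoveTerrain updates the counters and spawns another chunk whenever lanes drop below LaneMax.
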(event `self.ReceiveBeginPlay`
  (`self.MakeTerrain`))

(event `self.ReceiveTick`
  (params (DeltaSeconds :type "Float (single-precision)")))

(fn `GetRandomTerrain`
  (returns (Amount :type Integer))
  (set `self.LastTerrainIndex` (`KismetMathLibrary.RandomIntegerInRange` 0 2))
  (return (`KismetMathLibrary.RandomIntegerInRange` 0 2)))

(fn `MakeTerrain`
  (for _ (range 11)
    (`/Engine/EditorBlueprintResources/StandardMacros.IsValid` (`self.NewestTerrain`)
      (:`Is Valid`
        (`self.SpawnTerrainAtLocation` 0 true))
      (:`Is Not Valid`
        (`self.SpawnTerrain` (- (`self.K2_GetActorLocation` (`GameplayStatics.GetPlayerPawn` 0)) (495.0 500.0 40.0))))))
  (while (< (`self.LaneCount`) (`self.LaneMax`))
    (`self.SpawnTerrainChunk`)))

(fn `RemoveTerrain`
  (bind _lanecount (`self.LaneCount`))
  (`/Engine/EditorBlueprintResources/StandardMacros.IncrementInt` (`self.GenCount`)
    (:`  `
      (`/Engine/EditorBlueprintResources/StandardMacros.DecrementInt` _lanecount
        (:`  `
          (if (< _lanecount (`self.LaneMax`))
            (`self.SpawnTerrainChunk`)))))))

(fn `SpawnTerrain`
  (params (SpawnLocation :type "Vector Structure") (TerrainIndex :type Integer) (Init :type Boolean))
  (bind _returnvalue (`|SpawnActorFromClass` "/Game/ChickenRoad/Blueprints/Terrain.Terrain_C" (`KismetMathLibrary.MakeTransform` SpawnLocation) "AlwaysSpawn" "OverrideRootScale" null null))
  (`/Engine/EditorBlueprintResources/StandardMacros.IncrementInt` (`self.LaneCount`)
    (:`  `
      (bind _output_get (set `self.NewestTerrain` _returnvalue))
      (set `/Game/ChickenRoad/Blueprints/Terrain.TerrainGen` self _output_get)
      (`/Game/ChickenRoad/Blueprints/Terrain.PrepStaticMesh` _returnvalue TerrainIndex Init))))

(fn `SpawnTerrainAtLocation`
  (params (TerrainIndex :type Integer) (Init :type Boolean))
  (`self.SpawnTerrain` (`SceneComponent.K2_GetComponentLocation` (`/Game/ChickenRoad/Blueprints/Terrain.SpawnPoint` (`self.NewestTerrain`))) TerrainIndex Init))

(fn `SpawnTerrainChunk`
  (bind _amount (`self.GetRandomTerrain`))
  (for _ (range (+ _amount 1))
    (`self.SpawnTerrainAtLocation` (`self.LastTerrainIndex`))))

(fn `UserConstructionScript`)