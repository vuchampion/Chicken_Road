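; RR_Sign is a sign actor, likely a railroad signal, with two rect lights that alternate on and off.
; While Active, Tick calls SwitchLight every frame, which uses Switch to swap the lit side; the half-second Delay is never triggered.
; ToggleActive turns both lights off and clears Active, but its inactive branch only sets Switch, so it never reactivates the sign.
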(event `self.ReceiveTick`
  (params (DeltaSeconds :type "Float (single-precision)"))
  (if (`self.Active`)
    (`self.SwitchLight`)))

(fn `SwitchLight`
  (bind _rectlight (`self.RectLight`))
  (bind _rectlight1 (`self.RectLight1`))
  (if (`self.Active`)
    (if (`self.Switch`)
      (`LightComponent.SetIntensity` _rectlight 0.0)
      (`LightComponent.SetIntensity` _rectlight1 5000.0)
      (set `self.Switch` false)
      (else
        (`LightComponent.SetIntensity` _rectlight1 0.0)
        (`LightComponent.SetIntensity` _rectlight 5000.0)
        (set `self.Switch` true)))))

(fn `ToggleActive`
  (if (`self.Active`)
    (set `self.Active` false)
    (`LightComponent.SetIntensity` (`self.RectLight`) 0.0)
    (`LightComponent.SetIntensity` (`self.RectLight1`) 0.0)
    (else
      (set `self.Switch` true))))

(fn `UserConstructionScript`)