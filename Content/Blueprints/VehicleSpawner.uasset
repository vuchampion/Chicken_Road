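; Spawner actor that sends vehicles along a terrain strip, with direction and terrain type set by SpawnInitialVehicles, which also spawns the first one.
; Terrain index 3 gets a fixed high speed and spawn spacing, while others get a random speed.
; Each tick accumulates speed as distance, rolls against Rate at the spawn threshold, and offsets the counter by PrepVehicle's result after spawning.
; An exact distance match toggles the terrain's RRSign.
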(event `self.ReceiveTick`
  (params (DeltaSeconds :type "Float (single-precision)"))
  (`self.CheckSpawn`))

(fn `CheckSpawn`
  (bind _distance (`self.Distance`))
  (if (>= _distance (`self.SpawnDistance`))
    (set `self.Distance` 0.0)
    (if (<= (`KismetMathLibrary.RandomFloatInRange` 0.0 100.0) (`self.Rate`))
      (`self.SpawnVehicle` (`SceneComponent.K2_GetComponentLocation` (`self.DefaultSceneRoot`))))
    (else
      (set `self.Distance` (+ _distance (`self.VehicleSpeed`)))
      (if (== 110.0 _distance)
        (`/Game/ChickenRoad/Blueprints/RR_Sign.ToggleActive` (`/Game/ChickenRoad/Blueprints/Terrain.RRSign` (`self.Terrain`)))))))

(fn `PrepSpeed`
  (if (== (`self.TerrainIndex`) 3)
    (set `self.VehicleSpeed` 110.0)
    (set `self.SpawnDistance` 5500.0)
    (else
      (set `self.VehicleSpeed` (`KismetMathLibrary.RandomFloatInRange` 5.0 15.0)))))

(fn `SpawnInitialVehicles`
  (params (Direction :type Integer) (Terrain :type "/Game/ChickenRoad/Blueprints/Terrain Object Reference") (TerrainIndex :type Integer))
  (set `self.TerrainIndex` TerrainIndex)
  (set `self.Direction` Direction)
  (set `self.Terrain` Terrain)
  (`self.PrepSpeed`)
  (`self.SpawnVehicle` (`SceneComponent.K2_GetComponentLocation` (`self.DefaultSceneRoot`))))

(fn `SpawnVehicle`
  (params (Location :type "Vector Structure"))
  (bind _returnvalue (`|SpawnActorFromClass` "/Game/ChickenRoad/Blueprints/Vehicle.Vehicle_C" (`KismetMathLibrary.MakeTransform` Location) "Undefined" "OverrideRootScale" null null))
  (set `self.LastVehicle` _returnvalue)
  (bind _vehiclelength (`/Game/ChickenRoad/Blueprints/Vehicle.PrepVehicle` _returnvalue (`self.TerrainIndex`) (`self.Direction`) Location self (`self.VehicleSpeed`)))
  (set `self.Distance` (- 0.0 _vehiclelength)))

(fn `UserConstructionScript`)