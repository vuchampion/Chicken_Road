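; Terrain row actor for a lane-crossing game, dressed as grass, water, road or railroad.
; Each row picks a random end tile and hands it to TerrainGen as LastTile, keeping a connected path through grass obstacles.
; Water gets lily pads for short path shifts, otherwise a VehicleSpawner like roads and railroads; railroads add a sign.
; When the player leaves TriggerZone, it calls RemoveTerrain and destroys itself and its spawner.
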(event `self.ReceiveBeginPlay`)

(event `self.TriggerZone.OnComponentEndOverlap`
  (params (OverlappedComponent :type "PrimitiveComponent Object Reference") (OtherActor :type "Actor Object Reference") (OtherComp :type "PrimitiveComponent Object Reference") (OtherBodyIndex :type Integer))
  (cast `/Game/ChickenRoad/Blueprints/BPC_Player` OtherActor)
  (if (not (`self.Dead`))
    (set `self.Dead` true)
    (`/Game/ChickenRoad/Blueprints/TerrainGenerator.RemoveTerrain` (`self.TerrainGen`))
    (`/Engine/EditorBlueprintResources/StandardMacros.IsValid` (`self.Vspawner`)
      (:`Is Valid`
        (`self.K2_DestroyActor` (`self.Vspawner`)))
      (:`Is Not Valid`
        _))
    (`/Engine/EditorBlueprintResources/StandardMacros.IsValid` (`self.RRSign`)
      (:`Is Valid`
        _)
      (:`Is Not Valid`
        _))
    (`self.K2_DestroyActor`)))

(fn `InPath`
  (params (Index :type Integer))
  (returns (InPath :type Boolean))
  (bind _endtile (`self.EndTile`))
  (bind _lasttile (`/Game/ChickenRoad/Blueprints/TerrainGenerator.LastTile` (`self.TerrainGen`)))
  (if (`KismetMathLibrary.InRange_IntInt` Index 8 18)
    (return (`KismetMathLibrary.InRange_IntInt` Index (`KismetMathLibrary.Min` _lasttile _endtile) (`KismetMathLibrary.Max` _lasttile _endtile)))
    (else
      (return false))))

(fn `PlaceGrassObject`
  (bind _returnvalue (`KismetMathLibrary.RandomIntegerInRange` 0 3))
  (bind _treepos (`self.TreePos`))
  (if (== _returnvalue 0)
    (`InstancedStaticMeshComponent.AddInstance` (`self.Tree`) (`KismetMathLibrary.MakeTransform` _treepos (struct) (0.5 0.5 0.5)))
    (elif (== _returnvalue 1)
      (`InstancedStaticMeshComponent.AddInstance` (`self.Tree2`) (`KismetMathLibrary.MakeTransform` _treepos (struct) (0.5 0.5 0.5)))
      (elif (== _returnvalue 2)
        (`InstancedStaticMeshComponent.AddInstance` (`self.Rock`) (`KismetMathLibrary.MakeTransform` (`self.RockPos`)))
        (else
          (`InstancedStaticMeshComponent.AddInstance` (`self.Bush`) (`KismetMathLibrary.MakeTransform` _treepos (struct) (0.5 0.5 0.5))))))))

(fn `PlaceLilyPad`
  (`|SpawnActorFromClass` "/Game/ChickenRoad/Blueprints/Lilypad_Movement.Lilypad_Movement_C" (`KismetMathLibrary.MakeTransform` (+ (`SceneComponent.K2_GetComponentLocation` (`self.TerrainMeshCenter`)) (`self.LilyPos`))) "Undefined" "OverrideRootScale" null null))

(fn `PlaceRRSign`
  (bind _returnvalue (`|SpawnActorFromClass` "/Game/ChickenRoad/Blueprints/RR_Sign.RR_Sign_C" (`KismetMathLibrary.MakeTransform` (+ (`SceneComponent.K2_GetComponentLocation` (`self.TerrainMeshCenter`)) (`self.RRSignPos`))) "Undefined" "OverrideRootScale" null null))
  (set `self.RRSign` _returnvalue))

(fn `PrepSpawner`
  (bind _spawnhere (`self.SetSpawn`))
  (bind _returnvalue (`|SpawnActorFromClass` "/Game/ChickenRoad/Blueprints/VehicleSpawner.VehicleSpawner_C" (`KismetMathLibrary.MakeTransform` _spawnhere) "Undefined" "OverrideRootScale" null null))
  (set `self.Vspawner` _returnvalue)
  (`/Game/ChickenRoad/Blueprints/VehicleSpawner.SpawnInitialVehicles` _returnvalue (`self.Direction`) self (`self.TerrainIndex`)))

(fn `PrepStaticMesh`
  (params (TerrainIndex :type Integer) (Init :type Boolean))
  (bind _output_get (set `self.TerrainIndex` TerrainIndex))
  (`self.SetPath`)
  (if (== _output_get 0)
    (`self.SetGrassMesh` Init)
    (elif (== _output_get 1)
      (`self.SetWaterMesh`)
      (else
        (`self.SetRoadMesh`)))))

(fn `SetDirection`
  (params (TerrainIndex :type Integer))
  (if (!= TerrainIndex 0)
    (if (== TerrainIndex 1)
      (set `self.Direction` (`KismetMathLibrary.RandomIntegerInRange` -1 1))
      (else
        (set `self.Direction` (select `int` (`KismetMathLibrary.RandomIntegerInRange` 0 1) :`0` -1 :`1` 1))))))

(fn `SetFreeTile`)

(fn `SetGrassMesh`
  (params (Init :type Boolean))
  (`self.SetStaticMesh` 0)
  (`self.SetPath`)
  (for _index (range 27)
    (if Init
      (bind _returnvalue (`KismetMathLibrary.InRange_IntInt` _index 8 18))
      (if (not _returnvalue)
        (`self.PlaceGrassObject` :!label _label))
      (elif _returnvalue
        (bind _inpath (`self.InPath` _index))
        (if _inpath
          _
          (elif (<= 0.0 (`KismetMathLibrary.RandomFloatInRange` 0.0 100.0))
            (goto _label)
            (else
              _)))
        (else
          (goto _label))))
    (set `self.TreePos` (+ (`self.TreePos`) (110.0 0.0 0.0)))
    (set `self.RockPos` (+ (`self.RockPos`) (110.0 0.0 0.0))))
  (`self.UpdatePath`))

(fn `SetPath`
  (bind _lasttile (`/Game/ChickenRoad/Blueprints/TerrainGenerator.LastTile` (`self.TerrainGen`)))
  (bind _output_get (set `self.EndTile` (`KismetMathLibrary.RandomIntegerInRange` 8 18)))
  (if (< _output_get _lasttile)
    (set `self.Direction` -1)
    (elif (> _output_get _lasttile)
      (set `self.Direction` 1)
      (elif (<= (`self.TerrainIndex`) 1)
        (set `self.Direction` 0)))))

(fn `SetRoadMesh`
  (if (<= (`KismetMathLibrary.RandomFloatInRange` 0.0 100.0) 87.5)
    (bind _output_get (set `self.TerrainIndex` 2))
    (`self.SetStaticMesh` _output_get)
    (else
      (bind _output_get_2 (set `self.TerrainIndex` 3))
      (`self.SetStaticMesh` _output_get_2)
      (`self.PlaceRRSign`)))
  (`self.PrepSpawner`)
  (`self.UpdatePath`))

(fn `SetSpawn`
  (returns (SpawnHere :type "Vector Structure"))
  (if (== (`self.Direction`) 1)
    (return (`SceneComponent.K2_GetComponentLocation` (`self.SpawnA`)))
    (else
      (return (`SceneComponent.K2_GetComponentLocation` (`self.SpawnB`))))))

(fn `SetStaticMesh`
  (params (TerrainIndex :type Integer :default 0))
  (bind _staticmesh (`StaticMeshComponent.StaticMesh` (`self.TerrainMeshCenter`)))
  (`StaticMeshComponent.SetStaticMesh` (`self.TerrainMeshCenter`) (select `int` TerrainIndex :`0` "/Game/ChickenRoad/Assets/CR_Grass.CR_Grass" :`1` "/Game/ChickenRoad/Assets/CR_Water.CR_Water" :`2` "/Game/ChickenRoad/Assets/CR_Road.CR_Road" :`3` "/Game/ChickenRoad/Assets/CR_RRoad.CR_RRoad" :!type "StaticMesh Object Reference"))
  (`StaticMeshComponent.SetStaticMesh` (`self.TerrainMeshLeft`) _staticmesh)
  (`StaticMeshComponent.SetStaticMesh` (`self.TerrainMeshRight`) _staticmesh))

(fn `SetWaterMesh`
  (bind _output_get (set `self.TerrainIndex` 1))
  (`self.SetStaticMesh` _output_get)
  (if (`KismetMathLibrary.InRange_IntInt` (- (`/Game/ChickenRoad/Blueprints/TerrainGenerator.LastTile` (`self.TerrainGen`)) (`self.EndTile`)) -1 1)
    (for _index (range 27)
      (bind _inpath (`self.InPath` _index))
      (if _inpath
        (`self.PlaceLilyPad`))
      (set `self.LilyPos` (+ (110.0 0.0 0.0) (`self.LilyPos`))))
    (else
      (`self.PrepSpawner`)))
  (`self.UpdatePath`))

(fn `UpdatePath`
  (set `/Game/ChickenRoad/Blueprints/TerrainGenerator.LastTile` (`self.EndTile`) (`self.TerrainGen`)))

(fn `UserConstructionScript`)