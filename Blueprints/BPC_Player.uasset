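; Player Blueprint for a Crossy Road-style chicken that hops on a 110-unit grid, tracking furthest distance and coins.
; Directional inputs pass validity checks, then squash the mesh, jump, sweep-move the capsule and snap to grid, with forward hops updating distance.
; A per-frame idle timer, reset after move input, starts forward camera panning, then spawns an eagle that kills the chicken with sound and particles.
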(event `self.ReceiveTick`
  (params (DeltaSeconds :type "Float (single-precision)"))
  ;[1 1 1] Trigger Idle Death
  (`|ExecutionSequence`
    (:`then_0`
      (bind _result (`/Engine/EditorBlueprintResources/StandardMacros.IncrementInt` (`self.Timer`))
        (:`  `
          (if (== _result 600)
            (set `self.DeathByEagle` true)
            (`|SpawnActorFromClass` "/Game/Blueprints/Eagle.Eagle_C" (`KismetMathLibrary.MakeTransform` (+ (`SceneComponent.K2_GetComponentLocation` (`self.StaticMesh`)) (800.0 0.0 300.0)) (struct :`Yaw` 90.0)) "Undefined" "OverrideRootScale" null null)))))
    (:`then_1`
      (if (`self.DeathByEagle`)
        (set `self.IsDead` true)
        (`KismetSystemLibrary.Delay` 1.3)
        (`SceneComponent.SetRelativeScale3D` (`self.StaticMesh`) (0.0 0.0 0.0))
        (`GameplayStatics.SpawnSoundAttached` "/Game/Sounds/ChickenDeath.ChickenDeath" (`self.StaticMesh`) "None" (0.0 0.0 0.0) (struct) "KeepRelativeOffset" false 1.0 1.0 0.0 null null)
        (`GameplayStatics.SpawnEmitterAtLocation` "/Game/Particles/Water_Particles.Water_Particles" (`SceneComponent.K2_GetComponentLocation` (`self.StaticMesh`)))
        (set `self.DeathByEagle` false)
        (`KismetSystemLibrary.Delay` 1.0)
        (`self.K2_DestroyActor` (`self.Eagle`))))
    (:`then_2`
      (if (and (> (`self.Timer`) 150) (not (`self.IsDead`)))
        ;[1 1 1] Slow Camera Panning
        (`SceneComponent.K2_AddWorldOffset` (`self.Camera`) (`KismetMathLibrary.MakeVector` (* DeltaSeconds (`self.Pan Speed`))) false false)))))

(event `InputAction|Move Forward`
  (params (Key :type "Key Structure"))
  ;[1 1 1] Character Movement
  (:`Pressed`
    (bind _valid (`self.CheckValidity` (`self.R_Forward`)))
    (if _valid
      (set `self.IsJumping` true)
      (`self.Squish`)
      (`KismetSystemLibrary.Delay` 0.15)
      (`self.Unsquish`)
      (`self.Jump`)
      (`SceneComponent.K2_AddWorldOffset` (`self.CapsuleComponent`) (110.0 0.0 0.0) true false)
      (`self.CheckLocationHigh`))
    (`KismetSystemLibrary.Delay` 0.1)
    (`self.UpdateAfterJump`)))

(event `InputAction|Move Left`
  (params (Key :type "Key Structure"))
  ;[1 1 1] Character Movement
  (:`Pressed`
    (bind _valid (`self.CheckValidity` (`self.R_Left`)))
    (if _valid
      (set `self.IsJumping` true)
      (`self.Squish`)
      (`KismetSystemLibrary.Delay` 0.15)
      (`self.Unsquish`)
      (`self.Jump`)
      (`SceneComponent.K2_AddWorldOffset` (`self.CapsuleComponent`) (0.0 -110.0 0.0) true false))
    (`KismetSystemLibrary.Delay` 0.1)
    (`self.UpdateAfterJump`)))

(event `InputAction|Move Backward`
  (params (Key :type "Key Structure"))
  ;[1 1 1] Character Movement
  (:`Pressed`
    (bind _valid (`self.CheckValidity` (`self.R_Backward`)))
    (if _valid
      (set `self.IsJumping` true)
      (`self.Squish`)
      (`KismetSystemLibrary.Delay` 0.15)
      (`self.Unsquish`)
      (`self.Jump`)
      (`SceneComponent.K2_AddWorldOffset` (`self.CapsuleComponent`) (-110.0 0.0 0.0) true false))
    (`KismetSystemLibrary.Delay` 0.1)
    (`self.UpdateAfterJump`)))

(event `InputAction|Move Right`
  (params (Key :type "Key Structure"))
  ;[1 1 1] Character Movement
  (:`Pressed`
    (bind _valid (`self.CheckValidity` (`self.R_Right`)))
    (if _valid
      (set `self.IsJumping` true)
      (`self.Squish`)
      (`KismetSystemLibrary.Delay` 0.15)
      (`self.Unsquish`)
      (`self.Jump`)
      (`SceneComponent.K2_AddWorldOffset` (`self.CapsuleComponent`) (0.0 110.0 0.0) true false))
    (`KismetSystemLibrary.Delay` 0.1)
    (`self.UpdateAfterJump`)))

(event `self.ReceiveBeginPlay`
  ;[1 1 1] Camera Initialization
  (set `self.R_Forward` (`SceneComponent.K2_GetComponentRotation` (`self.StaticMesh`)))
  (`SceneComponent.SetAbsolute` (`self.Camera`) false false false))

(fn `Align`
  (bind (_returnvalue_x _returnvalue_y) (`KismetMathLibrary.BreakVector` (`SceneComponent.K2_GetComponentLocation` (`self.CapsuleComponent`))))
  (`SceneComponent.K2_SetWorldLocation` (`self.CapsuleComponent`) (`KismetMathLibrary.MakeVector` (* (`KismetMathLibrary.Round` (/ _returnvalue_x 110.0)) 110.0) (* (`KismetMathLibrary.Round` (/ _returnvalue_y 110.0)) 110.0)) false false))

(fn `CheckLocationHigh`
  (bind _furthestlocation_x (`KismetMathLibrary.BreakVector` (`self.FurthestLocation`)))
  (bind _returnvalue_x (`KismetMathLibrary.BreakVector` (`SceneComponent.K2_GetComponentLocation` (`self.StaticMesh`))))
  (if (> _returnvalue_x _furthestlocation_x)
    (`self.IncrementDistance`)))

(fn `CheckValidity`
  (params (`Chicken Orientation` :type "Rotator Structure"))
  (returns (Valid :type Boolean) (Invalid :type Boolean))
  (bind _staticmesh (`self.StaticMesh`))
  (`self.Align`)
  (if (`self.IsDead`)
    (return false true)
    (elif (`self.IsBlockedLeft`)
      (return false true)
      (elif (`self.IsBlockedRight`)
        (return false true)
        (elif (`self.IsJumping`)
          (return false true)
          (elif (not (== (`SceneComponent.K2_GetComponentRotation` _staticmesh) `Chicken Orientation`))
            (`SceneComponent.K2_SetWorldRotation` _staticmesh `Chicken Orientation` false false)
            (set `self.PreviousLocation` (`SceneComponent.K2_GetComponentLocation` (`self.CapsuleComponent`)))
            (return true false)))))))

(fn `IncrementCoin`
  (`/Engine/EditorBlueprintResources/StandardMacros.IncrementInt` (`self.Coins`)))

(fn `IncrementDistance`
  (bind _returnvalue_x (`KismetMathLibrary.BreakVector` (`SceneComponent.K2_GetComponentLocation` (`self.StaticMesh`))))
  (if (not (`self.IsDead`))
    (`/Engine/EditorBlueprintResources/StandardMacros.IncrementInt` (`self.Distance`)
      (:`  `
        (set `self.FurthestLocation` (`KismetMathLibrary.MakeVector` _returnvalue_x))))))

(fn `Squish`
  (`SceneComponent.SetRelativeScale3D` (`self.StaticMesh`) (1.2 1.0 0.65)))

(fn `Unsquish`
  (bind _staticmesh (`self.StaticMesh`))
  (`SceneComponent.SetRelativeScale3D` _staticmesh (1.0 1.0 1.0))
  (`GameplayStatics.SpawnSoundAttached` "/Game/Sounds/ChickenJump.ChickenJump" _staticmesh "None" (0.0 0.0 0.0) (struct) "KeepRelativeOffset" false 1.0 1.0 0.0 null null))

(fn `UpdateAfterJump`
  (set `self.IsJumping` false)
  (set `self.Timer` 0)
  (`self.Align`))

(fn `UserConstructionScript`)